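; Player-controlled wheeled van that drives at constant throttle with its rotation locked to zero and switches between three lanes, endless-runner style.
; Tick detects touch swipes over a distance threshold, once per press; left/right swipes or arrow keys pick a clamped lane.
; A timeline lerps the van's Y between lane positions via teleporting location updates rather than steering.
; Up/down swipes only print, and steering and handbrake calls are disconnected.
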(event EventTick
  (params (DeltaSeconds :type Float%20%28single-precision%29))
  (bind _returnvalue (Game|GetPlayerController 0))
  (bind _lane_y (Variables|Default|GetLane%20Y))
  (bind _mesh (Variables|Character|GetMesh))
  (bind (_locationx _locationy) (Class|PlayerController|GetInputTouchState _returnvalue "Touch1"))
  (bind _returnvalue_2 (Transformation|GetWorldLocation _mesh))
  (bind _returnvalue_3 (Math|Vector2D|MakeVector2D _locationx _locationy))
  ;[1 1 1] Touch Controller
  (Utilities|FlowControl|Sequence
    (:then_1
      (if (Variables|Default|GetisPressed)
        (if (> (Math|Vector2D|Vector2DLength (- (Variables|Default|GetTouch%20Start%202DVector) _returnvalue_3)) 1e+02)
          (Utilities|FlowControl|DoOnce false
            (:Completed
              (Variables|Default|SetTouch%20End%202DVector _returnvalue_3)
              (if (> (Math|Float|Absolute(Float) (.X (Math|Vector2D|BreakVector2D (- (Variables|Default|GetTouch%20Start%202DVector) (Variables|Default|GetTouch%20End%202DVector))))) (Math|Float|Absolute(Float) (.Y (Math|Vector2D|BreakVector2D (- (Variables|Default|GetTouch%20Start%202DVector) (Variables|Default|GetTouch%20End%202DVector))))))
                (if (> (.X (Math|Vector2D|BreakVector2D (- (Variables|Default|GetTouch%20Start%202DVector) (Variables|Default|GetTouch%20End%202DVector)))) 0.0)
                  (Development|PrintString "Left")
                  ;[1 1 1] controller
                  (Variables|Default|SetNewLane (Math|Integer|Clamp(Integer) (- (Variables|Default|Getlane) 1) 0 2))
                  (bind _laney (Timeline|Timeline_0 PlayFromStart)
                    (:Update
                      (Transformation|SetActorLocation (Math|Vector|MakeVector (.x _returnvalue_2) (Math|Float|Lerp (Utilities|Array|Get(acopy) _lane_y (Variables|Default|Getlane)) (Utilities|Array|Get(acopy) _lane_y (Variables|Default|GetNewLane)) _laney) (.z _returnvalue_2)) false true)
                      (Transformation|SetActorRotation "0, 0, 0"))
                    (:Finished
                      (Variables|Default|Setlane (Variables|Default|GetNewLane))))
                  (else
                    (Development|PrintString "Right")
                    (Variables|Default|SetNewLane (Math|Integer|Clamp(Integer) (- (Variables|Default|Getlane) -1) 0 2))
                    (Timeline|Timeline_0 PlayFromStart)))
                (elif (> (.Y (Math|Vector2D|BreakVector2D (- (Variables|Default|GetTouch%20Start%202DVector) (Variables|Default|GetTouch%20End%202DVector)))) 0.0)
                  (Development|PrintString "Up")
                  (else
                    (Development|PrintString "Down")))))))))))

(event EventBeginPlay)

(event Collision|EventActorBeginOverlap
  (params (OtherActor :type Actor%20Object%20Reference)))

(event Input|ActionEvents|InputActionFinger1
  (params (Key :type Key%20Structure))
  (bind _returnvalue (Game|GetPlayerController 0))
  (bind _lane_y (Variables|Default|GetLane%20Y))
  (bind _mesh (Variables|Character|GetMesh))
  (bind (_locationx _locationy) (Class|PlayerController|GetInputTouchState _returnvalue "Touch1"))
  (bind _returnvalue_2 (Transformation|GetWorldLocation _mesh))
  (bind _returnvalue_3 (Math|Vector2D|MakeVector2D _locationx _locationy))
  ;[1 1 1] Touch Controller
  (:Pressed
    (Variables|Default|SetisPressed true)
    (Variables|Default|SetTouch%20Start%202DVector _returnvalue_3))
  (:Released
    (Variables|Default|SetisPressed false)
    (Utilities|FlowControl|DoOnce false) ; enters at Reset
  ))

(event Input|ActionEvents|InputActionHandbrake
  (params (Key :type Key%20Structure))
  ;[1 1 1] Handbrake input
)

(event Input|AxisEvents|InputAxisMoveForward
  (params (AxisValue :type Float%20%28single-precision%29))
  ;[1 1 1] Throttle input
  (Class|WheeledVehicleMovementComponent|SetThrottleInput (Variables|Default|GetVehicleMovement) 1e+02)
  (Transformation|SetActorRotation "0, 0, 0" true))

(event Input|AxisEvents|InputAxisMoveRight
  (params (AxisValue :type Float%20%28single-precision%29))
  ;[1 1 1] Steering input
)

(event Input|KeyboardEvents|Left
  (params (Key :type Key%20Structure))
  (bind _lane_y (Variables|Default|GetLane%20Y))
  (bind _mesh (Variables|Character|GetMesh))
  (bind _returnvalue (Transformation|GetWorldLocation _mesh))
  ;[1 1 1] controller
  (:Pressed
    (Variables|Default|SetNewLane (Math|Integer|Clamp(Integer) (- (Variables|Default|Getlane) 1) 0 2))
    (bind _laney (Timeline|Timeline_0 PlayFromStart)
      (:Update
        (Transformation|SetActorLocation (Math|Vector|MakeVector (.x _returnvalue) (Math|Float|Lerp (Utilities|Array|Get(acopy) _lane_y (Variables|Default|Getlane)) (Utilities|Array|Get(acopy) _lane_y (Variables|Default|GetNewLane)) _laney) (.z _returnvalue)) false true)
        (Transformation|SetActorRotation "0, 0, 0"))
      (:Finished
        (Variables|Default|Setlane (Variables|Default|GetNewLane))))))

(event Input|KeyboardEvents|Right
  (params (Key :type Key%20Structure))
  (bind _lane_y (Variables|Default|GetLane%20Y))
  (bind _mesh (Variables|Character|GetMesh))
  (bind _returnvalue (Transformation|GetWorldLocation _mesh))
  ;[1 1 1] controller
  (:Pressed
    (Variables|Default|SetNewLane (Math|Integer|Clamp(Integer) (- (Variables|Default|Getlane) -1) 0 2))
    (bind _laney (Timeline|Timeline_0 PlayFromStart)
      (:Update
        (Transformation|SetActorLocation (Math|Vector|MakeVector (.x _returnvalue) (Math|Float|Lerp (Utilities|Array|Get(acopy) _lane_y (Variables|Default|Getlane)) (Utilities|Array|Get(acopy) _lane_y (Variables|Default|GetNewLane)) _laney) (.z _returnvalue)) false true)
        (Transformation|SetActorRotation "0, 0, 0"))
      (:Finished
        (Variables|Default|Setlane (Variables|Default|GetNewLane))))))

(fn ConstructionScript)